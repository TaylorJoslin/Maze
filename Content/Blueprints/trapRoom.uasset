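; Trap room actor that shuts a gate when an overlap hits its trigger box.
; A one-shot DoorClosed flag is set before the third-person character cast, so the first overlap of any actor consumes the trigger.
; For the player character, it plays a sound at the gate and runs the GatePos timeline.
; Each timeline update adds a scaled Z offset to the gate, accumulating movement rather than interpolating position.
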(event `self.Box.OnComponentBeginOverlap`
  (params (OverlappedComponent :type "PrimitiveComponent Object Reference") (OtherActor :type "Actor Object Reference") (OtherComp :type "PrimitiveComponent Object Reference") (OtherBodyIndex :type Integer) (bFromSweep :type Boolean) (SweepResult :type "HitResult Structure (by ref)"))
  (if (not (`self.doorClosed`))
    (set `self.doorClosed` true)
    (cast `/Game/ThirdPerson/Blueprints/BP_ThirdPersonCharacter` OtherActor)
    (`KismetSystemLibrary.PrintString` "TriggerHit")
    (`GameplayStatics.PlaySoundAtLocation` null (`SceneComponent.K2_GetComponentLocation` (`self.gate`)) (struct) 1.0 1.0 0.0 null null null null)
    (bind (_direction _gatezpos) (`Timeline|gatePos`)
      (:`Update`
        (`SceneComponent.K2_AddLocalOffset` (`self.gate`) (`KismetMathLibrary.MakeVector` 0.0 0.0 (* _gatezpos (`self.gateMoveDist`))) false false)))))

(fn `UserConstructionScript`)